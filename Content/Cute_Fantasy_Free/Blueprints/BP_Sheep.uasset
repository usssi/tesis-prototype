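; BP_Sheep is a sheep actor that tracks a love counter (AmorCount) and shows it visually.
; Each tick sets the FBCoras flipbook to the frame matching AmorCount, so it acts as a meter that addamorcount increments.
; The coras event enables and restarts the NgSCora Niagara effect, which has rendering turned off on BeginPlay.
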(event `self.ReceiveBeginPlay`
  (`NiagaraComponent.SetRenderingEnabled` (`self.NgS_Cora`) false))

(event `self.ReceiveTick`
  (params (DeltaSeconds :type "Float (single-precision)"))
  (`PaperFlipbookComponent.SetPlaybackPositionInFrames` (`self.FB_Coras`) (`self.AmorCount`) false))

(event `coras`
  (bind _ngs_cora (`self.NgS_Cora`))
  (`NiagaraComponent.SetRenderingEnabled` _ngs_cora true)
  (`NiagaraComponent.ReinitializeSystem` _ngs_cora))

(event `add amor count`
  (set `self.AmorCount` (+ (`self.AmorCount`) 1)))

(fn `UserConstructionScript`)