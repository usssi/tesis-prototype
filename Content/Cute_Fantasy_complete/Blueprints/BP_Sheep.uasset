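; BP_Sheep is a sheep character with sleep, idle and dance flipbooks, a love ("amor") counter and a heart particle effect.
; Tick polls IsSheepAwake, re-applying sleep (which zeroes love and selects the tutorial song) or using DoOnce gates per love level.
; Waking at zero love selects the sheep's song; higher levels advance the heart flipbook and trigger TLMP_Actor stages.
; Love gains update BP_MusicManager and the WB_LevelsMenu heart total.
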(event `self.ReceiveBeginPlay`
  (`NiagaraComponent.SetRenderingEnabled` (`self.NgS_Cora`) false)
  (`self.SheepSleeps`))

(event `self.ReceiveTick`
  (params (DeltaSeconds :type "Float (single-precision)"))
  (`self.OvejaStateController`))

(event `particulasCorazonesOveja`
  (bind _ngs_cora (`self.NgS_Cora`))
  (`NiagaraComponent.SetRenderingEnabled` _ngs_cora true)
  (`NiagaraComponent.ReinitializeSystem` _ngs_cora))

(event `add amor count`
  (bind _output_get (set `self.OvejaAmorCount` (+ (`self.OvejaAmorCount`) 1)))
  (bind _returnvalue (`GameplayStatics.GetActorOfClass` "/Game/Blueprints/BP_MusicManager.BP_MusicManager_C"))
  (set `/Game/Blueprints/BP_MusicManager.SheepLove` _output_get _returnvalue)
  (`self.addHeartToUItextCorazones`))

(event `SheepSleeps`
  (`PaperFlipbookComponent.SetFlipbook` (`self.FB_Sheep`) "/Game/Cute_Fantasy_complete/Animals/Sheep/FlipBooksSheep/sleeping/FB_SheepSleeping.FB_SheepSleeping")
  (`SceneComponent.SetHiddenInGame` (`self.FB_Coras`) true false)
  (set `self.OvejaAmorCount` 0)
  (bind _foundwidgets (`WidgetBlueprintLibrary.GetAllWidgetsOfClass` "/Game/Widget/WB_LevelsMenu.WB_LevelsMenu_C" false))
  (for _array_element _foundwidgets
    (set `/Game/Widget/WB_LevelButton.SongSequenceToPlay` (`self.TutorialOveja`) (`/Game/Widget/WB_LevelsMenu.WB_LevelButton_Oveja` _array_element))))

(event `SheepIdles`
  (`PaperFlipbookComponent.SetFlipbook` (`self.FB_Sheep`) "/Game/Cute_Fantasy_complete/Animals/Sheep/FlipBooksSheep/FB_SheepIdle.FB_SheepIdle")
  (`SceneComponent.SetHiddenInGame` (`self.FB_Coras`) false false)
  (bind _foundwidgets (`WidgetBlueprintLibrary.GetAllWidgetsOfClass` "/Game/Widget/WB_LevelsMenu.WB_LevelsMenu_C" false))
  (for _array_element _foundwidgets
    (set `/Game/Widget/WB_LevelButton.SongSequenceToPlay` (`self.Oveja`) (`/Game/Widget/WB_LevelsMenu.WB_LevelButton_Oveja` _array_element))))

(event `SheepDances`
  (`PaperFlipbookComponent.SetFlipbook` (`self.FB_Sheep`) "/Game/Cute_Fantasy_complete/Animals/Sheep/FlipBooksSheep/FB_SheepDance.FB_SheepDance")
  (`SceneComponent.SetHiddenInGame` (`self.FB_Coras`) false false))

(event `SetCorasLevelUI`
  (`PaperFlipbookComponent.SetPlaybackPositionInFrames` (`self.FB_Coras`) (+ (`self.OvejaAmorCount`) 1) false))

(event `OvejaStateController`
  (bind _ovejaamorcount (`self.OvejaAmorCount`))
  (if (`self.isSheepAwake`)
    (if (== _ovejaamorcount 0)
      (`/Engine/EditorBlueprintResources/StandardMacros.DoOnce` false
        (:`Completed`
          (`self.SheepIdles`)))
      (elif (== _ovejaamorcount 1)
        (`/Engine/EditorBlueprintResources/StandardMacros.DoOnce` false
          (:`Completed`
            (`self.SetCorasLevelUI`)
            (bind _astlmp_actor (castclass `/Game/Blueprints/TLMP_Actor` "/Game/Blueprints/TLMP_Actor.TLMP_Actor_C"))
            (bind _outactors (`GameplayStatics.GetAllActorsOfClass` _astlmp_actor))
            (for _array_element _outactors
              (`/Game/Blueprints/TLMP_Actor.ActivateSheepStuff1` _array_element))))
        (elif (== _ovejaamorcount 2)
          (`/Engine/EditorBlueprintResources/StandardMacros.DoOnce` false
            (:`Completed`
              (`self.SetCorasLevelUI`)
              (bind _astlmp_actor_2 (castclass `/Game/Blueprints/TLMP_Actor` "/Game/Blueprints/TLMP_Actor.TLMP_Actor_C"))
              (bind _outactors_2 (`GameplayStatics.GetAllActorsOfClass` _astlmp_actor_2))
              (for _array_element_2 _outactors_2
                (`/Game/Blueprints/TLMP_Actor.ActivateSheepStuff2` _array_element_2))))
          (elif (== _ovejaamorcount 3)
            (`/Engine/EditorBlueprintResources/StandardMacros.DoOnce` false
              (:`Completed`
                (`self.SetCorasLevelUI`)))))))
    (else
      (`self.SheepSleeps`))))

(event `addHeartToUItextCorazones`
  (bind _foundwidgets (`WidgetBlueprintLibrary.GetAllWidgetsOfClass` "/Game/Widget/WB_LevelsMenu.WB_LevelsMenu_C" false))
  (for _array_element _foundwidgets
    (set `/Game/Widget/WB_LevelsMenu.TextUICorazones` (+ (`/Game/Widget/WB_LevelsMenu.TextUICorazones` _array_element) 1) _array_element)))

(fn `UserConstructionScript`)