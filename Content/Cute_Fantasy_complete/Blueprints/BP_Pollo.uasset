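; Chicken (Pollo) character that sleeps until flagged awake and tracks a love count shown through heart flipbook, Niagara effect and wake-up UI.
; Tick polls a state controller: sleeping resets love and selects the tutorial song in WB_LevelsMenu, while waking switches to idle and the Pollo song.
; Love increments feed BP_MusicManager and the menu's heart total, mirrored in world text against the wake-up requirement.
; Higher love stages only update hearts and print placeholders.
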(event `self.ReceiveBeginPlay`
  (`NiagaraComponent.SetRenderingEnabled` (`self.NgS_Cora`) false)
  (`self.PolloSleeps`))

(event `self.ReceiveTick`
  (params (DeltaSeconds :type "Float (single-precision)"))
  (`self.PolloStateController`)
  (`self.TextSet`))

(event `particulasCorazonesPollo`
  (bind _ngs_cora (`self.NgS_Cora`))
  (`NiagaraComponent.SetRenderingEnabled` _ngs_cora true)
  (`NiagaraComponent.ReinitializeSystem` _ngs_cora))

(event `add amor count`
  (bind _output_get (set `self.PolloAmorCount` (+ (`self.PolloAmorCount`) 1)))
  (bind _returnvalue (`GameplayStatics.GetActorOfClass` "/Game/Blueprints/BP_MusicManager.BP_MusicManager_C"))
  (set `/Game/Blueprints/BP_MusicManager.PollitoLove` _output_get _returnvalue)
  (`self.addHeartToUItextCorazones`))

(event `PolloSleeps`
  (`PaperFlipbookComponent.SetFlipbook` (`self.FB_Pollo`) "/Game/Cute_Fantasy_complete/Animals/Chicken/polloFLipBooks/FB_sleepingpollo.FB_sleepingpollo")
  (`SceneComponent.SetHiddenInGame` (`self.FB_Coras`) true false)
  (`SceneComponent.SetHiddenInGame` (`self.UI wakeUP`) false false)
  (set `self.PolloAmorCount` 0)
  (bind _foundwidgets (`WidgetBlueprintLibrary.GetAllWidgetsOfClass` "/Game/Widget/WB_LevelsMenu.WB_LevelsMenu_C" false))
  (for _array_element _foundwidgets
    (set `/Game/Widget/WB_LevelButton.SongSequenceToPlay` (`self.TutorialPollo`) (`/Game/Widget/WB_LevelsMenu.WB_LevelButton_Pollos` _array_element))))

(event `PolloIdles`
  (`PaperFlipbookComponent.SetFlipbook` (`self.FB_Pollo`) "/Game/Cute_Fantasy_complete/Animals/Chicken/polloFLipBooks/FB_IdlePollo.FB_IdlePollo")
  (`SceneComponent.SetHiddenInGame` (`self.FB_Coras`) false false)
  (`SceneComponent.SetHiddenInGame` (`self.UI wakeUP`) true true)
  (bind _foundwidgets (`WidgetBlueprintLibrary.GetAllWidgetsOfClass` "/Game/Widget/WB_LevelsMenu.WB_LevelsMenu_C" false))
  (for _array_element _foundwidgets
    (set `/Game/Widget/WB_LevelButton.SongSequenceToPlay` (`self.Pollo`) (`/Game/Widget/WB_LevelsMenu.WB_LevelButton_Pollos` _array_element))))

(event `PolloDances`
  (`PaperFlipbookComponent.SetFlipbook` (`self.FB_Pollo`) "/Game/Cute_Fantasy_complete/Animals/Chicken/polloFLipBooks/FB_dancePollo.FB_dancePollo")
  (`SceneComponent.SetHiddenInGame` (`self.FB_Coras`) false false))

(event `SetCorasLevelUI`
  (bind _polloamorcount (`self.PolloAmorCount`))
  (`PaperFlipbookComponent.SetPlaybackPositionInFrames` (`self.FB_Coras`) (+ _polloamorcount 1) false)
  (`KismetSystemLibrary.PrintString` (`KismetStringLibrary.Conv_IntToString` _polloamorcount)))

(event `PolloStateController`
  (bind _polloamorcount (`self.PolloAmorCount`))
  (if (`self.isPolloAwake`)
    (if (== _polloamorcount 0)
      (`/Engine/EditorBlueprintResources/StandardMacros.DoOnce` false
        (:`Completed`
          (`self.PolloIdles`)))
      (elif (== _polloamorcount 1)
        (`/Engine/EditorBlueprintResources/StandardMacros.DoOnce` false
          (:`Completed`
            (`KismetSystemLibrary.PrintString` "POLLO WALKS AROUND THE FARM")
            (`self.SetCorasLevelUI`)))
        (elif (== _polloamorcount 2)
          (`/Engine/EditorBlueprintResources/StandardMacros.DoOnce` false
            (:`Completed`
              (`KismetSystemLibrary.PrintString` "POLLO goes drink wasser")
              (`self.SetCorasLevelUI`)))
          (elif (== _polloamorcount 3)
            (`/Engine/EditorBlueprintResources/StandardMacros.DoOnce` false
              (:`Completed`
                (`KismetSystemLibrary.PrintString` "ni puta idea de que pasa aca")
                (`self.SetCorasLevelUI`)))))))
    (else
      (`self.PolloSleeps`))))

(event `addHeartToUItextCorazones`
  (bind _foundwidgets (`WidgetBlueprintLibrary.GetAllWidgetsOfClass` "/Game/Widget/WB_LevelsMenu.WB_LevelsMenu_C" false))
  (for _array_element _foundwidgets
    (set `/Game/Widget/WB_LevelsMenu.TextUICorazones` (+ (`/Game/Widget/WB_LevelsMenu.TextUICorazones` _array_element) 1) _array_element)))

(event `TextSet`
  (bind _foundwidgets (`WidgetBlueprintLibrary.GetAllWidgetsOfClass` "/Game/Widget/WB_LevelsMenu.WB_LevelsMenu_C" false))
  (for _array_element _foundwidgets
    (`TextRenderComponent.K2_SetText` (`self.TextRender`) (`|FormatText` "{currentHeart}/{neededHearts}" (`/Game/Widget/WB_LevelsMenu.TextUICorazones` _array_element) (`self.NeededCoraToWakeUpPollo`)))))

(fn `UserConstructionScript`)