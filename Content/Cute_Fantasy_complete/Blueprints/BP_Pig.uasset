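; Paper2D pig character that sleeps until IsPigAwake is set, tracking love hearts that feed the music manager and levels menu.
; Tick polls its state, using DoOnce gates to update the heart flipbook and trigger TLMP_Actor stages one and two.
; Sleep and idle switch the pig's menu song between TutorialPig and Pig.
; A text render shows menu hearts against the wake-up requirement, recolored when they match.
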(event `self.ReceiveBeginPlay`
  (`NiagaraComponent.SetRenderingEnabled` (`self.NgS_Cora`) false)
  (`self.PigSleeps`))

(event `self.ReceiveTick`
  (params (DeltaSeconds :type "Float (single-precision)"))
  (`self.PigStateController`)
  (`self.TextSet`)
  (`self.SetTextColor`))

(event `particulasCorazonesPig`
  (bind _ngs_cora (`self.NgS_Cora`))
  (`NiagaraComponent.SetRenderingEnabled` _ngs_cora true)
  (`NiagaraComponent.ReinitializeSystem` _ngs_cora))

(event `add amor count`
  (bind _output_get (set `self.PigAmorCount` (+ (`self.PigAmorCount`) 1)))
  (bind _returnvalue (`GameplayStatics.GetActorOfClass` "/Game/Blueprints/BP_MusicManager.BP_MusicManager_C"))
  (set `/Game/Blueprints/BP_MusicManager.PigLove` _output_get _returnvalue)
  (`self.addHeartToUItextCorazones`))

(event `PigSleeps`
  (`PaperFlipbookComponent.SetFlipbook` (`self.FB_Pig`) "/Game/Cute_Fantasy_complete/Animals/Pig/PigFlipBooks/FB_PigSleep.FB_PigSleep")
  (`SceneComponent.SetHiddenInGame` (`self.FB_Coras`) true false)
  (`SceneComponent.SetHiddenInGame` (`self.UI wakeUP`) false false)
  (set `self.PigAmorCount` 0)
  (bind _foundwidgets (`WidgetBlueprintLibrary.GetAllWidgetsOfClass` "/Game/Widget/WB_LevelsMenu.WB_LevelsMenu_C" false))
  (for _array_element _foundwidgets
    (set `/Game/Widget/WB_LevelButton.SongSequenceToPlay` (`self.TutorialPig`) (`/Game/Widget/WB_LevelsMenu.WB_LevelButton_Pig` _array_element))))

(event `PigIdles`
  (`PaperFlipbookComponent.SetFlipbook` (`self.FB_Pig`) "/Game/Cute_Fantasy_complete/Animals/Pig/PigFlipBooks/FB_pigIdle.FB_pigIdle")
  (`SceneComponent.SetHiddenInGame` (`self.FB_Coras`) false false)
  (`SceneComponent.SetHiddenInGame` (`self.UI wakeUP`) true true)
  (bind _foundwidgets (`WidgetBlueprintLibrary.GetAllWidgetsOfClass` "/Game/Widget/WB_LevelsMenu.WB_LevelsMenu_C" false))
  (for _array_element _foundwidgets
    (set `/Game/Widget/WB_LevelButton.SongSequenceToPlay` (`self.Pig`) (`/Game/Widget/WB_LevelsMenu.WB_LevelButton_Pig` _array_element))))

(event `PigDances`
  (`PaperFlipbookComponent.SetFlipbook` (`self.FB_Pig`) "/Game/Cute_Fantasy_complete/Animals/Pig/PigFlipBooks/FB_PigDance.FB_PigDance")
  (`SceneComponent.SetHiddenInGame` (`self.FB_Coras`) false false))

(event `SetCorasLevelUI`
  (`PaperFlipbookComponent.SetPlaybackPositionInFrames` (`self.FB_Coras`) (+ (`self.PigAmorCount`) 1) false))

(event `PigStateController`
  (bind _pigamorcount (`self.PigAmorCount`))
  (if (`self.isPigAwake`)
    (if (== _pigamorcount 0)
      (`/Engine/EditorBlueprintResources/StandardMacros.DoOnce` false
        (:`Completed`
          (`self.PigIdles`)))
      (elif (== _pigamorcount 1)
        (`/Engine/EditorBlueprintResources/StandardMacros.DoOnce` false
          (:`Completed`
            (`self.SetCorasLevelUI`)
            (bind _astlmp_actor (castclass `/Game/Blueprints/TLMP_Actor` "/Game/Blueprints/TLMP_Actor.TLMP_Actor_C"))
            (bind _outactors (`GameplayStatics.GetAllActorsOfClass` _astlmp_actor))
            (for _array_element _outactors
              (`/Game/Blueprints/TLMP_Actor.ActivatePigStuff1` _array_element))))
        (elif (== _pigamorcount 2)
          (`/Engine/EditorBlueprintResources/StandardMacros.DoOnce` false
            (:`Completed`
              (`self.SetCorasLevelUI`)
              (bind _astlmp_actor_2 (castclass `/Game/Blueprints/TLMP_Actor` "/Game/Blueprints/TLMP_Actor.TLMP_Actor_C"))
              (bind _outactors_2 (`GameplayStatics.GetAllActorsOfClass` _astlmp_actor_2))
              (for _array_element_2 _outactors_2
                (`/Game/Blueprints/TLMP_Actor.ActivatePigStuff2` _array_element_2))))
          (elif (== _pigamorcount 3)
            (`/Engine/EditorBlueprintResources/StandardMacros.DoOnce` false
              (:`Completed`
                (`self.SetCorasLevelUI`)))))))
    (else
      (`self.PigSleeps`))))

(event `addHeartToUItextCorazones`
  (bind _foundwidgets (`WidgetBlueprintLibrary.GetAllWidgetsOfClass` "/Game/Widget/WB_LevelsMenu.WB_LevelsMenu_C" false))
  (for _array_element _foundwidgets
    (set `/Game/Widget/WB_LevelsMenu.TextUICorazones` (+ (`/Game/Widget/WB_LevelsMenu.TextUICorazones` _array_element) 1) _array_element)))

(event `TextSet`
  (bind _foundwidgets (`WidgetBlueprintLibrary.GetAllWidgetsOfClass` "/Game/Widget/WB_LevelsMenu.WB_LevelsMenu_C" false))
  (for _array_element _foundwidgets
    (`TextRenderComponent.K2_SetText` (`self.TextRender`) (`|FormatText` "{currentHeart}/{neededHearts}" (`/Game/Widget/WB_LevelsMenu.TextUICorazones` _array_element) (`self.NeededCoraToWakeUpPig`)))))

(event `SetTextColor`
  (bind _textrender (`self.TextRender`))
  (bind _foundwidgets (`WidgetBlueprintLibrary.GetAllWidgetsOfClass` "/Game/Widget/WB_LevelsMenu.WB_LevelsMenu_C" false))
  (for _array_element _foundwidgets
    (if (== (`/Game/Widget/WB_LevelsMenu.TextUICorazones` _array_element) (`self.NeededCoraToWakeUpPig`))
      (`TextRenderComponent.SetTextRenderColor` _textrender (`self.ColorForReady`))
      (else
        (`TextRenderComponent.SetTextRenderColor` _textrender (`self.Color for Not`))))))

(fn `UserConstructionScript`)