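; BP_GrassAnimation toggles the visibility of its Animationgrass1 component based on the active camera and the sheep's state.
; Every Tick it looks up BP_CameraManager and BP_Sheep with GetActorOfClass rather than caching references.
; The grass animation shows only while CameraIndex is 0 and the sheep is not awake, and is hidden on any other camera.
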(event `self.ReceiveTick`
  (params (DeltaSeconds :type "Float (single-precision)"))
  (bind _asbp_camera_manager (castclass `/Game/Blueprints/BP_CameraManager` "/Game/Blueprints/BP_CameraManager.BP_CameraManager_C"))
  (bind _returnvalue (`GameplayStatics.GetActorOfClass` _asbp_camera_manager))
  (bind _returnvalue_2 (== (`/Game/Blueprints/BP_CameraManager.cameraIndex` _returnvalue) 0))
  (`SceneComponent.SetVisibility` (`self.animationgrass1`) _returnvalue_2 false)
  (if _returnvalue_2
    (bind _asbp_sheep (castclass `/Game/Cute_Fantasy_complete/Blueprints/BP_Sheep` "/Game/Cute_Fantasy_complete/Blueprints/BP_Sheep.BP_Sheep_C"))
    (bind _returnvalue_3 (`GameplayStatics.GetActorOfClass` _asbp_sheep))
    (`SceneComponent.SetVisibility` (`self.animationgrass1`) (not (`/Game/Cute_Fantasy_complete/Blueprints/BP_Sheep.isSheepAwake` _returnvalue_3)) false)))

(fn `UserConstructionScript`)