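; TLMP_Actor is a farm scenery actor that reveals sheep, pig and chicken enclosures in two stages per animal.
; Six custom events toggle Hidden In Game on its components: stage one shows each animal's fence.
; Stage two adds decor for sheep and pigs, but swaps the chicken fence for a coop.
; It has no active Tick, BeginPlay or construction logic, so the events must be triggered externally.
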(event `ActivateSheepStuff1`
  (`SceneComponent.SetHiddenInGame` (`self.TLM_FenceSheep`) false false))

(event `ActivateSheepStuff2`
  (`SceneComponent.SetHiddenInGame` (`self.TLMP_SheepDecor`) false false))

(event `ActivatePigStuff1`
  (`SceneComponent.SetHiddenInGame` (`self.TLM_FencePig`) false false))

(event `ActivatePigStuff2`
  (`SceneComponent.SetHiddenInGame` (`self.TLMP_PigDecor`) false false))

(event `ActivatePolloStuff1`
  (`SceneComponent.SetHiddenInGame` (`self.TLMP_ChickenFence`) false false))

(event `ActivatePolloStuff2`
  (`SceneComponent.SetHiddenInGame` (`self.TLMP_ChickenFence`) true false)
  (`SceneComponent.SetHiddenInGame` (`self.TLMP_ChickenCoop`) false false))

(fn `UserConstructionScript`)